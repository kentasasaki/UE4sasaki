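; PNPlayerPawn is the player character, with camera-relative movement, look controls, hold-to-sprint and a coin counter.
; Sprint switches max walk speed between the walk and sprint values.
; The first damage of any amount prints a death message, disables movement and sets a short lifespan, guarded by DoOnce.
; AddCoin and GetNumOfCoins expose the coin count, while the C key increments and prints it directly.
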(event `self.ReceiveBeginPlay`
  (set `CharacterMovementComponent.MaxWalkSpeed` (`self.GroundWalkSpeed`) (`self.CharacterMovement`)))

(event `InputAxis|MoveForward`
  (params (AxisValue :type "Float (single-precision)"))
  ;[1 1 1] 移動
  (`self.AddMovementInput` (`SceneComponent.GetForwardVector` (`self.Camera`)) AxisValue))

(event `InputAxis|LookUp`
  (params (AxisValue :type "Float (single-precision)"))
  ;[1 1 1] カメラ移動
  (`self.AddControllerPitchInput` AxisValue))

(event `self.ReceiveTick`
  (params (DeltaSeconds :type "Float (single-precision)")))

(event `InputAxis|LookRight`
  (params (AxisValue :type "Float (single-precision)"))
  ;[1 1 1] カメラ移動
  (`self.AddControllerYawInput` AxisValue))

(event `InputAxis|MoveRight`
  (params (AxisValue :type "Float (single-precision)"))
  ;[1 1 1] 移動
  (`self.AddMovementInput` (`SceneComponent.GetRightVector` (`self.Camera`)) AxisValue))

(event `self.ReceiveAnyDamage`
  (params (Damage :type "Float (single-precision)") (DamageType :type "DamageType Object Reference") (InstigatedBy :type "Controller Object Reference") (DamageCauser :type "Actor Object Reference"))
  ;[1 1 1] ダメージ
  (`/Engine/EditorBlueprintResources/StandardMacros.DoOnce` false ; 一度しかこの処理実行しない
    (:`Completed`
      (`KismetSystemLibrary.PrintString` "died" true true (struct :`R` 1.0 :`G` 0.199001 :`B` 0.237213 :`A` 1.0))
      (`CharacterMovementComponent.DisableMovement` (`self.CharacterMovement`))
      (`self.SetLifeSpan` 5.0))))

(event `InputAction|Sprint`
  (params (Key :type "Key Structure" :default "AnyKey"))
  (bind _charactermovement (`self.CharacterMovement`))
  ;[1 1 1] 移動速度が速くなる
  (:`Pressed`
    (set `CharacterMovementComponent.MaxWalkSpeed` (`self.GroundSpringSpeed`) _charactermovement))
  (:`Released`
    (set `CharacterMovementComponent.MaxWalkSpeed` (`self.GroundWalkSpeed`) _charactermovement)))

(event `Key|C`
  (params (Key :type "Key Structure" :default "AnyKey"))
  (:`Pressed`
    (bind _output_get (set `self.NumOfCoins` (+ (`self.NumOfCoins`) 1))) ; コイン枚数＝コイン枚数＋１
    (`KismetSystemLibrary.PrintString` (`KismetStringLibrary.Conv_IntToString` _output_get))))

(fn `AddCoin`
  (params (Num :type Integer))
  (set `self.NumOfCoins` (+ (`self.NumOfCoins`) Num)) ; コイン枚数＝コイン枚数＋１
)

(fn `GetNumOfCoins`
  (returns (ReturnValue :type Integer))
  (return (`self.NumOfCoins`)))

(fn `UserConstructionScript`)